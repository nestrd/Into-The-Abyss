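; Actor component that lets its owner act as a quest giver when the player interacts with it.
; On interaction it asks the player character's quest log whether its configured quest is active, printing "Quest in Progress" if so.
; Otherwise it looks up the quest's data table row and opens a quest giver widget with that data and ID.
; The interaction returns the owner's display name.
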(fn `DisplayQuest`
  (bind (_questdata_datatable _questdata_rowname) (break `DataTableRowHandle` (`self.QuestData`)))
  (bind _returnvalue (`|GetDataTableRow` _questdata_datatable _questdata_rowname)
    (:`then`
      (bind _returnvalue_2 (`|CreateWidget` "/Game/Systems/Quests/UI/WBP_QuestGiver.WBP_QuestGiver_C" null _returnvalue _questdata_rowname null))
      (`UserWidget.AddToViewport` _returnvalue_2 0))))

(fn `I_InteractWith`
  (returns (ObjectiveID :type String))
  (bind (_questdata_datatable _questdata_rowname) (break `DataTableRowHandle` (`self.QuestData`)))
  (bind _returnvalue (`KismetSystemLibrary.GetDisplayName` (`self.GetOwner`)))
  (if (not (`/Game/Systems/Quests/AC_QuestLog.QueryActiveQuest` (`/Game/Characters/Player/New/Character/BP_Character.AC_QuestLog` (`/Game/Systems/Quests/CommonFunctionLibrary.GetMyPlayerCharacter`)) _questdata_rowname))
    (`self.DisplayQuest`)
    (return _returnvalue)
    (else
      (`KismetSystemLibrary.PrintString` "Quest in Progress")
      (return _returnvalue))))