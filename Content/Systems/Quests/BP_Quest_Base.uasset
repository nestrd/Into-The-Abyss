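; BP_Quest_Base is a base quest actor that tracks objective progress for the current stage of a quest.
; On BeginPlay it loads its row from DT_QuestData by QuestID, seeds a progress map with the current stage's objectives at zero, and binds to the player character's objective-ID event.
; Its objective handler increments a matching objective's count until it reaches that objective's required quantity; no stage advancement is implemented here.
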(event `self.ReceiveBeginPlay`
  (`self.GetQuestData`)
  (add `/Game/Characters/Player/New/Character/BP_Character.OnObjectiveIDCalled` (`/Game/Systems/Quests/CommonFunctionLibrary.GetMyPlayerCharacter`) (`|CreateDelegate` :!event `On Objective IDHeard`)))

(fn `GetObjectiveDataFromID`
  (params (ObjectiveID :type String))
  (returns (ObjectiveData :type "/Game/Systems/Quests/FObjectiveData Structure"))
  (for _array_element (`.Objectives_24_39F9F89F4215C5F743BD32B909B24C8B` (break `/Game/Systems/Quests/FStageData` (`self.CurrrentStageData`)))
    (if (`KismetStringLibrary.EqualEqual_StrStr` (`.ObjectiveID_21_B8EBF44048311E303F6215A2FD38E55F` (break `/Game/Systems/Quests/FObjectiveData` _array_element)) (`local.ObjectiveID`))
      (return _array_element))))

(fn `GetQuestData`
  (bind _returnvalue (`|GetDataTableRow` "/Game/Systems/Quests/DT_QuestData.DT_QuestData" (`self.QuestID`))
    (:`then`
      (bind _output_get (set `self.QuestData` _returnvalue))
      (bind _output_get_2 (set `self.CurrrentStageData` (`|GetArrayItem` (`.Stages_15_F1CC0F374435EFF3C5E1C1BA5A0A9FE3` (break `/Game/Systems/Quests/FQuestData` _output_get)) (`self.CurrentStageNumber`))))
      (`BlueprintMapLibrary.Map_Clear` (`self.CurrentObjectiveProgress`))
      (for _array_element (`.Objectives_24_39F9F89F4215C5F743BD32B909B24C8B` (break `/Game/Systems/Quests/FStageData` _output_get_2))
        (`BlueprintMapLibrary.Map_Add` (`self.CurrentObjectiveProgress`) (`.ObjectiveID_21_B8EBF44048311E303F6215A2FD38E55F` (break `/Game/Systems/Quests/FObjectiveData` _array_element)))))))

(fn `On Objective IDHeard`
  (params (ObjectiveID :type String))
  (bind (_value _returnvalue) (`BlueprintMapLibrary.Map_Find` (`self.CurrentObjectiveProgress`) ObjectiveID))
  (if _returnvalue
    (if (< _value (`.Quantity_12_8478FAD94F7564009B58FFB0754A4668` (break `/Game/Systems/Quests/FObjectiveData` (`self.GetObjectiveDataFromID` ObjectiveID))))
      (`BlueprintMapLibrary.Map_Add` (`self.CurrentObjectiveProgress`) (`local.ObjectiveID`) (+ _value 1))
      (else
        (return)))
    (else
      (return))))

(fn `UserConstructionScript`)