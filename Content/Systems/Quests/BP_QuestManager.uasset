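; Quest manager that tracks started and completed quests in a map from quest data to a completion flag.
; StartQuest ignores quests already in the map, otherwise fires OnQuestStarted and prints quest details, while CompleteQuest fires OnQuestCompleted and sets the flag.
; ProgressQuest delegates to the quest data object itself.
; BeginPlay holds hardcoded test logic that starts DA_TargetTest, then progresses the first tracked quest after a short delay.
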(event `self.ReceiveBeginPlay`
  (`self.StartQuest` "/Game/Systems/Quests/DA_TargetTest.DA_TargetTest")
  (`KismetSystemLibrary.Delay` 3.0)
  (bind _keys (`BlueprintMapLibrary.Map_Keys` (`self.CompleteQuestList`)))
  (`self.ProgressQuest` (`|GetArrayItem` _keys)))

(event `StartQuest`
  (params (QuestData :type "/Game/Systems/Quests/PDA_Quest_Base Object Reference"))
  (if (not (`.ReturnValue` (`BlueprintMapLibrary.Map_Find` (`self.CompleteQuestList`) QuestData)))
    (`self.OnQuestStarted` QuestData)
    (`BlueprintMapLibrary.Map_Add` (`self.CompleteQuestList`) QuestData)
    (`KismetSystemLibrary.PrintString` (`KismetTextLibrary.Conv_TextToString` (`|FormatText` "Name = {QuestName} \nDescription = {Quest Description} \nQuest Type =  {Quest Type}" (`/Game/Systems/Quests/PDA_Quest_Base.QuestName` QuestData) (`/Game/Systems/Quests/PDA_Quest_Base.QuestDescription` QuestData) (`|GetEnumeratorNameAsString` (`/Game/Systems/Quests/PDA_Quest_Base.QuestType` QuestData)))) true true (struct :`G` 0.66 :`B` 1.0 :`A` 1.0) 10.0)))

(event `CompleteQuest`
  (params (`Quest Data` :type "/Game/Systems/Quests/PDA_Quest_Base Object Reference"))
  (`self.OnQuestCompleted` `Quest Data`)
  (`BlueprintMapLibrary.Map_Add` (`self.CompleteQuestList`) `Quest Data` true))

(event `ProgressQuest`
  (params (QuestData :type "/Game/Systems/Quests/PDA_Quest_Base Object Reference"))
  (`/Game/Systems/Quests/PDA_Quest_Base.ProgressQuest` QuestData))

(fn `UserConstructionScript`)