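; BP_DebugTextOnTiles is a debug visual aid that draws each grid tile's X,Y ID as floating text over the tile.
; It finds BP_GridManager on BeginPlay and binds to its tile-updated and grid-destroyed dispatchers.
; Text render actors are spawned on demand, cached in a map by tile ID and removed for missing tiles.
; SetShowTileIDs either labels every tile or destroys all cached text actors.
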(event `self.ReceiveBeginPlay`
  ;[1 1 1] Gets the BP_GridManager in the current level
  (bind _returnvalue (`GameplayStatics.GetActorOfClass` "/Game/Systems/GridSystem/BaseGrid/BP_GridManager.BP_GridManager_C"))
  (bind _output_get (set `self.Grid` _returnvalue))
  ;[1 1 1] Binds to the Tile update dispatcher so text renders are updated when the tile data changes
  (add `/Game/Systems/GridSystem/BaseGrid/BP_GridManager.OnTileDataUpdated` _output_get (`|CreateDelegate` :!event `UpdateTextOnTile`))
  ;[1 1 1] Binds to the Grid Destroyed dispatcher so it destroys all text debugs when the grid is cleared
  (add `/Game/Systems/GridSystem/BaseGrid/BP_GridManager.OnGridDestroyed` _output_get (`|CreateDelegate` :!event `ClearAllTextActors`)))

(fn `ClearAllTextActors`
  (bind _values (`BlueprintMapLibrary.Map_Values` (`self.TextRender_Library`)))
  (for _array_element _values
    (`self.K2_DestroyActor` _array_element))
  (`BlueprintMapLibrary.Map_Clear` (`self.TextRender_Library`)))

(fn `DestroyTextActor`
  (params (ID :type "IntPoint Structure"))
  (locals (`Text Render Actor To Destroy` :type "TextRenderActor Object Reference"))
  ;[1 1 1] Checks to see if the text render actor we want to destroy currently exists
  (bind _output_get (set `local.Text Render Actor To Destroy` (`BlueprintMapLibrary.Map_Find` (`self.TextRender_Library`) ID)))
  (`/Engine/EditorBlueprintResources/StandardMacros.IsValid` _output_get
    (:`Is Valid`
      (`self.K2_DestroyActor` _output_get)
      (`BlueprintMapLibrary.Map_Remove` (`self.TextRender_Library`) (`local.ID`)))))

(fn `GetTextActor`
  (params (ID :type "IntPoint Structure"))
  (returns (`Text Render Actor` :type "TextRenderActor Object Reference"))
  (locals (PossibleTextRender :type "TextRenderActor Object Reference"))
  (bind _possibletextrender (`local.PossibleTextRender`))
  (bind _textrender (`TextRenderActor.TextRender` (`local.PossibleTextRender`)))
  ;[1 1 1] Checks if we already have a text render actor for this tile before we try making one
  (bind _output_get (set `local.PossibleTextRender` (`BlueprintMapLibrary.Map_Find` (`self.TextRender_Library`) ID)))
  (`/Engine/EditorBlueprintResources/StandardMacros.IsValid` _output_get
    (:`Is Valid`
      ;[1 1 1] Epic and cool! We already have one and can leave early! POGGERS
      (return (`local.PossibleTextRender`)))
    (:`Is Not Valid`
      ;[1 1 1] Spawns a text render actor for our current tile and adds it to our library for later use
      (bind _returnvalue (`|SpawnActorFromClass` "/Script/Engine.TextRenderActor" (`KismetMathLibrary.MakeTransform` (0.0 0.0 0.0)) "AlwaysSpawn" "MultiplyWithRoot" null null))
      (bind _output_get_2 (set `local.PossibleTextRender` _returnvalue))
      (`BlueprintMapLibrary.Map_Add` (`self.TextRender_Library`) (`local.ID`) _output_get_2)
      ;[1 1 1] Sets our new Text Render Actor's settings
      (`self.SetActorTickEnabled` _possibletextrender false)
      (`self.SetActorEnableCollision` _possibletextrender false)
      (`TextRenderComponent.SetHorizontalAlignment` _textrender "EHTA_Center")
      (`TextRenderComponent.SetVerticalAlignment` _textrender "EVRTA_TextCenter")
      ;[1 1 1] We are done creating this text rendder actor and leave
      (return (`local.PossibleTextRender`)))))

(fn `SetShowTileIDs`
  (params (`Show Tile IDs` :type Boolean))
  (bind _output_get (set `self.ShowTileIDs` `Show Tile IDs`))
  (if _output_get
    (bind _keys (`BlueprintMapLibrary.Map_Keys` (`/Game/Systems/GridSystem/BaseGrid/BP_GridManager.Tile_Data_Library` (`self.Grid`))))
    (for _array_element _keys
      (`self.UpdateTextOnTile` _array_element))
    (else
      (`self.ClearAllTextActors`))))

(fn `UpdateTextOnTile`
  (params (`Tile ID` :type "IntPoint Structure"))
  (locals (CurrentTileData :type "/Game/Systems/GridSystem/BaseGrid/TileData/ST_TileData Structure") (CurrentTextRenderActor :type "TextRenderActor Object Reference") (DisplayText :type String))
  (bind (_tile_id_x _tile_id_y) (break `IntPoint` (`local.Tile ID`)))
  (bind (_value _returnvalue) (`BlueprintMapLibrary.Map_Find` (`/Game/Systems/GridSystem/BaseGrid/BP_GridManager.Tile_Data_Library` (`self.Grid`)) `Tile ID`))
  (if (`self.ShowTileIDs`)
    ;[1 1 1] Try and find the tile we want to change text for
    (if _returnvalue
      ;[1 1 1] Tile is valid, so we get the tile data and it's text render actor
      (set `local.CurrentTileData` _value)
      (bind _text_render_actor (`self.GetTextActor` (`local.Tile ID`)))
      (set `local.CurrentTextRenderActor` _text_render_actor)
      ;[1 1 1] Set the text render actor's display text
      (set `local.DisplayText` (`KismetStringLibrary.Concat_StrStr` (`KismetStringLibrary.Conv_IntToString` _tile_id_x) ", " (`KismetStringLibrary.Conv_IntToString` _tile_id_y)))
      ;[1 1 1] Update the Text Render's actual Text
      (`TextRenderComponent.K2_SetText` (`TextRenderActor.TextRender` (`local.CurrentTextRenderActor`)) (`KismetTextLibrary.Conv_StringToText` (`local.DisplayText`)))
      ;[1 1 1] Update the text render's transform to match it's matching tile
      (`self.K2_SetActorTransform` (`local.CurrentTextRenderActor`) (`KismetMathLibrary.MakeTransform` (+ (.location (`.Transform_12_ACB12EFD46E1A6A0191A1C9C09D4F5A4` (break `/Game/Systems/GridSystem/BaseGrid/TileData/ST_TileData` (`local.CurrentTileData`)))) (0.0 0.0 1.0)) (struct :`Pitch` 90.0 :`Yaw` 180.0) (2.0 2.0 2.0)) false false)
      (else
        ;[1 1 1] If we can't find then tile then destroy it's text render actor
        (`self.DestroyTextActor` `Tile ID`)))))

(fn `UserConstructionScript`)