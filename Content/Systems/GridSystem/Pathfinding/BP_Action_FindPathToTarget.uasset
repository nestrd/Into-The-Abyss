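; Grid debug action that finds a path from the debug pawn's selected tile to a target tile and marks it on the grid.
; Execution clears two tile states, binds to the pathfinding completion event, then calls FindPath on the grid's pathfinding component with diagonal, iteration-delay and per-frame time-budget settings.
; The completion callback adds the path state to each returned tile.
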(fn `Execute Action`
  (params (`Tile ID` :type "IntPoint Structure"))
  (bind _griddebugpawn (`self.GridDebugPawn`))
  ;[0 0 0] This grid action is designed to show tile neighbours on the grid
  ;;[0 0 0] Clears the grid of any previous Is Neighbour States we activated
  (`/Game/Systems/GridSystem/BaseGrid/BFL_GridUtilities.ClearStateFromAllTiles` "NewEnumerator7" (`/Game/Systems/GridSystem/DebugTools/BP_GridDebugPawn.BP_Grid` (`self.GridDebugPawn`)))
  (`/Game/Systems/GridSystem/BaseGrid/BFL_GridUtilities.ClearStateFromAllTiles` "NewEnumerator8" (`/Game/Systems/GridSystem/DebugTools/BP_GridDebugPawn.BP_Grid` (`self.GridDebugPawn`)))
  ;;[0 0 0] Adds the IsPath state to all of our Path Tiles
  (add `/Game/Systems/GridSystem/Pathfinding/BP_GridPathfinding.OnPathfindingCompleted` (`/Game/Systems/GridSystem/BaseGrid/BP_GridManager.Grid_Pathfinding` (`/Game/Systems/GridSystem/DebugTools/BP_GridDebugPawn.BP_Grid` (`self.GridDebugPawn`))) (`|CreateDelegate` :!event `OnPathfindingCompleted`))
  ;;[0 0 0] Gets all of our input tile's valid neighbours from the Grid Pathfinding BP
  (`/Game/Systems/GridSystem/Pathfinding/BP_GridPathfinding.FindPath` (`/Game/Systems/GridSystem/BaseGrid/BP_GridManager.Grid_Pathfinding` (`/Game/Systems/GridSystem/DebugTools/BP_GridDebugPawn.BP_Grid` _griddebugpawn)) (`/Game/Systems/GridSystem/DebugTools/BP_GridDebugPawn.SelectedTile` _griddebugpawn) `Tile ID` (`self.Include Diagonals`) (`self.DelayBetweenIterations`) (`self.MaxMSPerFrame`)))

(fn `OnPathfindingCompleted`
  (params (Array :type "Array of IntPoint Structure"))
  (for _array_element Array
    (`/Game/Systems/GridSystem/BaseGrid/BFL_GridUtilities.Add State To Tile` _array_element "NewEnumerator8" (`/Game/Systems/GridSystem/DebugTools/BP_GridDebugPawn.BP_Grid` (`self.GridDebugPawn`)))))

(fn `UserConstructionScript`
  (`parent.UserConstructionScript`))