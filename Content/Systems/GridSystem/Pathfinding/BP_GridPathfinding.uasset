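; Grid pathfinding Blueprint that runs A* over BPGrid tiles to find a path for characters, filtered by allowed terrain types.
; FindPath expands the cheapest tile from a cost-sorted discovered array, applying terrain entry costs and a diagonal tie-break, then walks PreviousIDs back to build the path.
; It runs synchronously or, given a delay, time-sliced under a per-frame millisecond budget.
; Dispatcher calls report data updates, clears and completion.
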(event `FindPathWithDelay`
  (`|ExecutionSequence`
    (:`then_0`
      (goto _label_3 :!via `Open`))
    (:`then_1`
      (set `self.LoopStartTime` (`KismetMathLibrary.Now`) :!label _label)
      ;[0 0 0] Checks if we have discovered any possible tiles
      (if (> (`KismetArrayLibrary.Array_Length` (`self.DiscoveredTileIDs`)) 0) :!label _label_2
        ;[0 0 0] Analyses each discovered tile one by one until we find the target tile
        (bind _foundtargettile (`self.AnalyseNextDiscoveredTile`))
        (if _foundtargettile
          ;[0 0 0] Takes our analysed tile list and returns a valid path for our character to follow
          (bind _path (`self.GeneratePath`))
          (`self.OnPathfindingCompleted` _path)
          (else
            (if (> (`self.MaxMSPerFrame`) 0.0)
              (if (< (`KismetMathLibrary.GetTotalMilliseconds` (- (`KismetMathLibrary.Now`) (`self.LoopStartTime`))) (`self.MaxMSPerFrame`))
                (goto _label_2)
                (else
                  _)))
            (`KismetSystemLibrary.RetriggerableDelay` (`self.DelayBetweenIterations`))
            (`/Engine/EditorBlueprintResources/StandardMacros.Gate` true :!label _label_3
              (:`Exit`
                (goto _label)))))
        (else
          ;[0 0 0] No Possible Path
          (`self.OnPathfindingCompleted` (`|MakeArray` (struct) :!type "IntPoint Structure")))))))

(event `CloseDelayGate`
  (goto _label_3 :!via `Close`))

(fn `AnalyseNextDiscoveredTile`
  (returns (FoundTargetTile :type Boolean))
  ;[0 0 0] We are pulling the cheapest tile out of the discovered list and moving it to the analysed list. This leaves the discovered list empty, ready for us to add our analysed tile's neighbours
  (bind _tilepathdata (`self.PullCheapestTileOutOfDiscoveredList`))
  (bind _output_get (set `self.CurrentDiscoveredTile` _tilepathdata))
  (`self.OnPathfindingDataUpdated` (`.ID_2_4C0497C148304509A23CB49C19C1FAEB` (break `/Game/Systems/GridSystem/Pathfinding/ST_PathfindingData` _output_get)))
  ;[0 0 0] Here we are getting our analysed tile's neighbours
  (bind _valid_neighbours (`self.Get Valid Tile Neighbours` (`.ID_2_4C0497C148304509A23CB49C19C1FAEB` (break `/Game/Systems/GridSystem/Pathfinding/ST_PathfindingData` (`self.CurrentDiscoveredTile`))) (`self.IncludeDiagonals`) (`self.Valid Tile Types`)))
  (set `self.CurrentNeighbours` _valid_neighbours)
  (while (> (`KismetArrayLibrary.Array_Length` (`self.CurrentNeighbours`)) 0)
    ;[0 0 0] We are checking if any of the neighbour tiles are the target tile
    (bind _istargettile (`self.DiscoverNextNeighbour`))
    (if _istargettile
      ;[0 0 0] This neighbour is the target and we have a path
      (return true)))
  ;[0 0 0] None of the neighbours were the target tile
  (return false))

(fn `ClearGeneratedData`
  (`BlueprintMapLibrary.Map_Clear` (`self.PathfindingData`))
  (`KismetArrayLibrary.Array_Clear` (`self.DiscoveredTileSortingCosts`))
  (`KismetArrayLibrary.Array_Clear` (`self.DiscoveredTileIDs`))
  (`KismetArrayLibrary.Array_Clear` (`self.AnalysedTileIDs`))
  (`self.OnPathfindingDataCleared`))

(fn `DiscoverNextNeighbour`
  (returns (IsTargetTile :type Boolean))
  (locals (CostFromStart :type Integer) (IndexInDiscovered :type Integer :default 0))
  (bind _indexindiscovered (`local.IndexInDiscovered`))
  (bind (_id _costtoentertile) (break `/Game/Systems/GridSystem/Pathfinding/ST_PathfindingData` (`self.CurrentNeighbour`)))
  ;[0 0 0] Pulling the current neighbour we want to discover out of the neighbour array
  (set `self.CurrentNeighbour` (`|GetArrayItem` (`self.CurrentNeighbours`)))
  (`KismetArrayLibrary.Array_Remove` (`self.CurrentNeighbours`))
  ;[0 0 0] Checking if we have already analysed the current neighbour
  (if (not (`KismetArrayLibrary.Array_Contains` (`self.AnalysedTileIDs`) (`.ID_2_4C0497C148304509A23CB49C19C1FAEB` (break `/Game/Systems/GridSystem/Pathfinding/ST_PathfindingData` (`self.CurrentNeighbour`)))))
    ;[0 0 0] Calculating the cost from start for this tile, this will be helpful for determing character movement range.
    (set `local.CostFromStart` (+ (`.CostFromStart_7_EB916F3645C58443D8085FAD52EB14A2` (break `/Game/Systems/GridSystem/Pathfinding/ST_PathfindingData` (`self.CurrentDiscoveredTile`))) (`.CostToEnterTile_5_6168ED08445ED885657C13B36181AAA3` (break `/Game/Systems/GridSystem/Pathfinding/ST_PathfindingData` (`self.CurrentNeighbour`)))))
    ;[0 0 0] Checks if we have previously discovered this tile, if we haave then this tile is already known to be valid, if not then we can continue with an null reference
    (bind _output_get (set `local.IndexInDiscovered` (`KismetArrayLibrary.Array_Find` (`self.DiscoveredTileIDs`) (`.ID_2_4C0497C148304509A23CB49C19C1FAEB` (break `/Game/Systems/GridSystem/Pathfinding/ST_PathfindingData` (`self.CurrentNeighbour`))))))
    (if (not (== _output_get -1))
      ;[0 0 0] Here we are checking if we have found a faster route to the neighbour tile
      ;;[0 0 0] We are loading the pre-existing pathfinding data for the tile so we can compare it to the new route
      (bind _output_get_2 (set `self.CurrentNeighbour` (`BlueprintMapLibrary.Map_Find` (`self.PathfindingData`) (`.ID_2_4C0497C148304509A23CB49C19C1FAEB` (break `/Game/Systems/GridSystem/Pathfinding/ST_PathfindingData` (`self.CurrentNeighbour`))))))
      (if (< (`local.CostFromStart`) (`.CostFromStart_7_EB916F3645C58443D8085FAD52EB14A2` (break `/Game/Systems/GridSystem/Pathfinding/ST_PathfindingData` _output_get_2)))
        ;[0 0 0] We have found a new faster route, so we are deleting our prior data for this tile ready to update it
        (`KismetArrayLibrary.Array_Remove` (`self.DiscoveredTileIDs`) _indexindiscovered)
        (`KismetArrayLibrary.Array_Remove` (`self.DiscoveredTileSortingCosts`) _indexindiscovered)
        (else
          ;[0 0 0] There is already a faster route to this tile so we should early out
          (return false))))
    ;[0 0 0] We go discover mode and pass through the relevant tile data
    (`self.DiscoverTile` (make `/Game/Systems/GridSystem/Pathfinding/ST_PathfindingData` _id _costtoentertile (`local.CostFromStart`) (`self.GetMinimumCostBetweenTwoTiles` (`.ID_2_4C0497C148304509A23CB49C19C1FAEB` (break `/Game/Systems/GridSystem/Pathfinding/ST_PathfindingData` (`self.CurrentNeighbour`))) (`self.TargetID`) (`self.IncludeDiagonals`)) (`.ID_2_4C0497C148304509A23CB49C19C1FAEB` (break `/Game/Systems/GridSystem/Pathfinding/ST_PathfindingData` (`self.CurrentDiscoveredTile`)))))
    ;[0 0 0] Finally we check if this tile ID is the same as the target tile and return
    (if (`KismetMathLibrary.Equal_IntPointIntPoint` (`.ID_2_4C0497C148304509A23CB49C19C1FAEB` (break `/Game/Systems/GridSystem/Pathfinding/ST_PathfindingData` (`self.CurrentNeighbour`))) (`self.TargetID`))
      (return true)
      (else
        (return false)))
    (else
      ;[0 0 0] We already analysed this tile and we should early out
      (return false))))

(fn `DiscoverTile`
  (params (TilePathData :type "/Game/Systems/GridSystem/Pathfinding/ST_PathfindingData Structure"))
  (bind _id (break `/Game/Systems/GridSystem/Pathfinding/ST_PathfindingData` TilePathData))
  (`BlueprintMapLibrary.Map_Add` (`self.PathfindingData`) _id TilePathData)
  (`self.InsertTileInDiscoveredArray` TilePathData)
  (`self.OnPathfindingDataUpdated` _id))

(fn `FindPath`
  (params (Start :type "IntPoint Structure") (Target :type "IntPoint Structure") (Diagonals :type Boolean) (Delay :type "Float (double-precision)") (MaxMS :type "Float (double-precision)") (`Tile Types` :type "Array of /Game/Systems/GridSystem/BaseGrid/TileData/EN_TileTerrain Enum"))
  (returns (Path :type "Array of IntPoint Structure"))
  (bind _array (`|MakeArray` (struct) :!type "IntPoint Structure"))
  (bind _array_2 (`|MakeArray` (struct) :!type "IntPoint Structure"))
  ;[0 0 0] This function is the core of our pathfinding algorithm and is meant to be called by characters for moving along the grid. If you want to learn how the algorithm works, this is the best starting point
  ;;[0 0 0] Set variables so we can access them later for debugging and visualizing the pathfinding process
  (set `self.StartID` Start)
  (set `self.TargetID` Target)
  (set `self.IncludeDiagonals` Diagonals)
  (set `self.Valid Tile Types` `Tile Types`)
  (set `self.DelayBetweenIterations` Delay)
  (set `self.MaxMSPerFrame` MaxMS)
  (`self.CloseDelayGate`)
  ;;[0 0 0] Clears data from prior Pathfinding queries
  (`self.ClearGeneratedData`)
  ;;[0 0 0] Checks that our input variables (StartID, TargetID) are valid grid coordinates
  (bind _is_valid (`self.InInputDataValid?`))
  (if _is_valid
    ;;[0 0 0] Adds Start Tile to the discovered list because we now know that it is a valid grid position
    (`self.DiscoverTile` (make `/Game/Systems/GridSystem/Pathfinding/ST_PathfindingData` (`self.StartID`) 1 0 (`self.GetMinimumCostBetweenTwoTiles` (`self.StartID`) (`self.TargetID`) (`self.IncludeDiagonals`))))
    ;;[0 0 0] Checks if we want to use a delay during our pathfinding query
    (if (<= (`self.DelayBetweenIterations`) 0.0)
      ;;[0 0 0] Checks if we have discovered any possible tiles
      (while (> (`KismetArrayLibrary.Array_Length` (`self.DiscoveredTileIDs`)) 0)
        ;;[0 0 0] Analyses each discovered tile one by one until we find the target tile
        (bind _foundtargettile (`self.AnalyseNextDiscoveredTile`))
        (if _foundtargettile
          ;;[0 0 0] Takes our analysed tile list and returns a valid path for our character to follow
          (bind _path (`self.GeneratePath`))
          (`self.OnPathfindingCompleted` _path)
          (return _path)))
      ;;[0 0 0] No Possible Path
      (`self.OnPathfindingCompleted` _array)
      (return _array)
      (else
        (`self.FindPathWithDelay`)
        (return (`|MakeArray` (struct) :!type "IntPoint Structure"))))
    (else
      ;;[0 0 0] Some or all of the inputs aren't valid so we are returning an empty Array
      (`self.OnPathfindingCompleted` _array_2)
      (return _array_2))))

(fn `GeneratePath`
  (returns (Path :type "Array of IntPoint Structure"))
  (locals (Current :type "IntPoint Structure") (InvertedPath :type "Array of IntPoint Structure") (ReturnArray :type "Array of IntPoint Structure"))
  (set `local.Current` (`self.TargetID`))
  (while (!= (`local.Current`) (`self.StartID`))
    (`KismetArrayLibrary.Array_Add` (`local.InvertedPath`) (`local.Current`))
    (set `local.Current` (`.PreviousID_12_CF7C13D541DABB534F4D83A290084441` (break `/Game/Systems/GridSystem/Pathfinding/ST_PathfindingData` (`BlueprintMapLibrary.Map_Find` (`self.PathfindingData`) (`local.Current`))))))
  (bind (_arrayindex _arrayelement) (`/Engine/EditorBlueprintResources/StandardMacros.ReverseForEachLoop` (`local.InvertedPath`))
    (:`LoopBody`
      (`KismetArrayLibrary.Array_Add` (`local.ReturnArray`) _arrayelement))
    (:`Completed`
      (return (`local.ReturnArray`)))))

(fn `Get Tile Neighbours`
  (params (`Tile ID` :type "IntPoint Structure") (`Include Diagonals` :type Boolean))
  (returns (Neighbours :type "Array of IntPoint Structure"))
  (locals (`Return Neighbour Array` :type "Array of IntPoint Structure"))
  (bind _array (`|MakeArray` (+ (`local.Tile ID`) (make `IntPoint` 1)) (+ (`local.Tile ID`) (make `IntPoint` 0 1)) (+ (`local.Tile ID`) (make `IntPoint` -1)) (+ (`local.Tile ID`) (make `IntPoint` 0 -1))))
  ;[0 0 0] This function takes our input tile's grid ID and gets it's surrounding tiles as an array.
  ;;[0 0 0] Checks if we want to get diagonal neighbours or not?
  (if `Include Diagonals`
    ;;[0 0 0] Calls non diagonal neighbours and places them in an array
    (bind _output_get (set `local.Return Neighbour Array` _array))
    ;;[0 0 0] Gets our input tile's diagonal neighbour's and appens them to the Return Neighbour Array
    (`KismetArrayLibrary.Array_Append` _output_get (`|MakeArray` (+ (`local.Tile ID`) (make `IntPoint` 1 1)) (+ (`local.Tile ID`) (make `IntPoint` -1 1)) (+ (`local.Tile ID`) (make `IntPoint` -1 -1)) (+ (`local.Tile ID`) (make `IntPoint` 1 -1))))
    ;;[0 0 0] Returns with both direct and diagonal neighbours
    (return (`local.Return Neighbour Array`))
    (else
      ;;[0 0 0] Returns with only direct neighbours
      (return _array))))

(fn `Get Valid Tile Neighbours`
  (params (ID :type "IntPoint Structure") (`Include Diagonals` :type Boolean) (`Valid Types` :type "Array of /Game/Systems/GridSystem/BaseGrid/TileData/EN_TileTerrain Enum"))
  (returns (`Valid Neighbours` :type "Array of /Game/Systems/GridSystem/Pathfinding/ST_PathfindingData Structure"))
  (locals (`Tile Data` :type "/Game/Systems/GridSystem/BaseGrid/TileData/ST_TileData Structure") (`Input Tile Data` :type "/Game/Systems/GridSystem/BaseGrid/TileData/ST_TileData Structure") (`Return Neighbour Array` :type "Array of /Game/Systems/GridSystem/Pathfinding/ST_PathfindingData Structure"))
  (bind (_tile_data_tileid _tile_data_tilestates _tile_data_transform _tile_data_visited _tile_data_walkable_ _tile_data_terrain) (break `/Game/Systems/GridSystem/BaseGrid/TileData/ST_TileData` (`local.Tile Data`)))
  ;[0 0 0] This Function checks for validated neighbours, it's the bigger, beefier version of 'GetTileNeighbours' and is designed for character pathfinding. This means if you want to just edit the raw tiles, it's probably overkill and you should use 'GetTileNeighbours'.
  ;;[0 0 0] Checks that our input tile ID is valid and gets it's tile data for future comparisons with it's neighbours
  (set `local.Input Tile Data` (`BlueprintMapLibrary.Map_Find` (`/Game/Systems/GridSystem/BaseGrid/BP_GridManager.Tile_Data_Library` (`self.BP_Grid`)) ID))
  ;;[0 0 0] Gets our tile's raw neighbours for validating
  (for _array_element (`self.Get Tile Neighbours` ID `Include Diagonals`)
    (bind (_value _returnvalue) (`BlueprintMapLibrary.Map_Find` (`/Game/Systems/GridSystem/BaseGrid/BP_GridManager.Tile_Data_Library` (`self.BP_Grid`)) _array_element))
    ;;[0 0 0] Gets the neighbour tile and checks that it is a valid tile in our grid, then saves it's tile data for comparison
    (bind _output_get (set `local.Tile Data` _value))
    (if _returnvalue
      (if (`KismetArrayLibrary.Array_Contains` `Valid Types` (`.Terrain_24_E629DEFF45AA8E6AB9C870A32B4167DD` (break `/Game/Systems/GridSystem/BaseGrid/TileData/ST_TileData` _output_get)))
        ;;[0 0 0] Saves all the valid tile neighbours to our return array
        (`KismetArrayLibrary.Array_Add` (`local.Return Neighbour Array`) (make `/Game/Systems/GridSystem/Pathfinding/ST_PathfindingData` _tile_data_tileid (select `/Game/Systems/GridSystem/BaseGrid/TileData/EN_TileTerrain` _tile_data_terrain :`NewEnumerator0` 1 :`NewEnumerator11` 2 :`NewEnumerator12` 3 :`NewEnumerator13` 1 :`NewEnumerator14` 99999) 99999 99999 ID)))))
  ;;[0 0 0] Returns our validated Neighbours
  (return (`local.Return Neighbour Array`)))

(fn `GetMinimumCostBetweenTwoTiles`
  (params (`Tile ID 1` :type "IntPoint Structure") (`Tile ID 2` :type "IntPoint Structure") (Diagonals :type Boolean))
  (returns (`Min Cost` :type Integer))
  (bind (_returnvalue_x _returnvalue_y) (break `IntPoint` (- `Tile ID 1` `Tile ID 2`)))
  (bind (_returnvalue_x_2 _returnvalue_y_2) (break `IntPoint` (- `Tile ID 1` `Tile ID 2`)))
  (if Diagonals
    (return (`KismetMathLibrary.Max` (`KismetMathLibrary.Abs_Int` _returnvalue_x_2) (`KismetMathLibrary.Abs_Int` _returnvalue_y_2)))
    (else
      (return (+ (`KismetMathLibrary.Abs_Int` _returnvalue_x) (`KismetMathLibrary.Abs_Int` _returnvalue_y))))))

(fn `GetTileSortingCost`
  (params (ST_PathfindingData :type "/Game/Systems/GridSystem/Pathfinding/ST_PathfindingData Structure (by ref)"))
  (returns (ReturnValue :type Integer))
  (bind (_id _costtoentertile _costfromstart _minimumcosttotarget) (break `/Game/Systems/GridSystem/Pathfinding/ST_PathfindingData` ST_PathfindingData))
  (bind (_id_2 _costtoentertile_2 _costfromstart_2 _minimumcosttotarget_2 _previousid) (break `/Game/Systems/GridSystem/Pathfinding/ST_PathfindingData` ST_PathfindingData))
  (return (+ (* (+ _costfromstart _minimumcosttotarget) 2) (`self.IsDiagonal` _id_2 _previousid))))

(fn `InInputDataValid?`
  (returns (`Is Valid` :type Boolean))
  (if (!= (`self.StartID`) (`self.TargetID`))
    (if (`/Game/Systems/GridSystem/BaseGrid/BP_GridManager.IsTileWalkable` (`self.BP_Grid`) (`self.StartID`))
      (if (`/Game/Systems/GridSystem/BaseGrid/BP_GridManager.IsTileWalkable` (`self.BP_Grid`) (`self.TargetID`))
        (if (`KismetArrayLibrary.Array_Contains` (`self.Valid Tile Types`) (`.Terrain_24_E629DEFF45AA8E6AB9C870A32B4167DD` (break `/Game/Systems/GridSystem/BaseGrid/TileData/ST_TileData` (`BlueprintMapLibrary.Map_Find` (`/Game/Systems/GridSystem/BaseGrid/BP_GridManager.Tile_Data_Library` (`self.BP_Grid`)) (`self.TargetID`)))))
          (return true)
          (else
            (return false)))
        (else
          (return false)))
      (else
        (return false)))
    (else
      (return false))))

(fn `InsertTileInDiscoveredArray`
  (params (TileData :type "/Game/Systems/GridSystem/Pathfinding/ST_PathfindingData Structure"))
  (locals (SortingCost :type Integer))
  (bind _discoveredtilesortingcosts (`self.DiscoveredTileSortingCosts`))
  (set `local.SortingCost` (`self.GetTileSortingCost` TileData))
  (if (== (`KismetArrayLibrary.Array_Length` (`self.DiscoveredTileSortingCosts`)) 0)
    (`KismetArrayLibrary.Array_Add` (`self.DiscoveredTileSortingCosts`) (`local.SortingCost`) :!label _label)
    (`KismetArrayLibrary.Array_Add` (`self.DiscoveredTileIDs`) (`.ID_2_4C0497C148304509A23CB49C19C1FAEB` (break `/Game/Systems/GridSystem/Pathfinding/ST_PathfindingData` TileData)))
    (elif (>= (`local.SortingCost`) (`|GetArrayItem` _discoveredtilesortingcosts (`KismetArrayLibrary.Array_LastIndex` _discoveredtilesortingcosts)))
      (goto _label)
      (else
        (for (_array_element _array_index) (`self.DiscoveredTileSortingCosts`)
          (if (>= _array_element (`local.SortingCost`))
            (`KismetArrayLibrary.Array_Insert` (`self.DiscoveredTileSortingCosts`) (`local.SortingCost`) _array_index)
            (`KismetArrayLibrary.Array_Insert` (`self.DiscoveredTileIDs`) (`.ID_2_4C0497C148304509A23CB49C19C1FAEB` (break `/Game/Systems/GridSystem/Pathfinding/ST_PathfindingData` TileData)) _array_index)
            (break)))))))

(fn `IsDiagonal`
  (params (`ID 1` :type "IntPoint Structure") (`ID 2` :type "IntPoint Structure"))
  (returns (IsDiagonal :type Boolean))
  (return (not (`KismetArrayLibrary.Array_Contains` (`self.Get Tile Neighbours` `ID 1`) `ID 2`))))

(fn `PullCheapestTileOutOfDiscoveredList`
  (returns (TilePathData :type "/Game/Systems/GridSystem/Pathfinding/ST_PathfindingData Structure"))
  (locals (TileID :type "IntPoint Structure"))
  ;[0 0 0] This is a pretty simple function that pulls the cheapest discovered tile into the analysed list for analysing
  ;;[0 0 0] We get the first Index of the Discovered Tile IDs Array, this array has already been filtered so the cheapest tile is first so we can safely pull from 0
  (set `local.TileID` (`|GetArrayItem` (`self.DiscoveredTileIDs`)))
  ;;[0 0 0] We remove the Tile index  from the discovered list in preperation for it being added to the Analysed List
  (`KismetArrayLibrary.Array_Remove` (`self.DiscoveredTileSortingCosts`))
  (`KismetArrayLibrary.Array_Remove` (`self.DiscoveredTileIDs`))
  ;;[0 0 0] We add the tile to the analysed list
  (`KismetArrayLibrary.Array_Add` (`self.AnalysedTileIDs`) (`local.TileID`))
  ;;[0 0 0] Returns the Pathfinding Data for using in analysing the tile
  (return (`BlueprintMapLibrary.Map_Find` (`self.PathfindingData`) (`local.TileID`))))

(fn `UserConstructionScript`)