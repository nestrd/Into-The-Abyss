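; A debug grid action that highlights the valid neighbours of a given tile.
; Execute Action clears the neighbour state and two other tile states from the grid, then asks the grid's pathfinding component for neighbours, filtered by allowed tile types and optionally including diagonals.
; Each returned tile receives the neighbour state on the grid referenced by the debug pawn.
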(fn `Execute Action`
  (params (`Tile ID` :type "IntPoint Structure"))
  ;[0 0 0] This grid action is designed to show tile neighbours on the grid
  ;;[0 0 0] Clears the grid of any previous Is Neighbour States we activated
  (`/Game/Systems/GridSystem/BaseGrid/BFL_GridUtilities.ClearStateFromAllTiles` "NewEnumerator2" (`/Game/Systems/GridSystem/DebugTools/BP_GridDebugPawn.BP_Grid` (`self.GridDebugPawn`)))
  (`/Game/Systems/GridSystem/BaseGrid/BFL_GridUtilities.ClearStateFromAllTiles` "NewEnumerator8" (`/Game/Systems/GridSystem/DebugTools/BP_GridDebugPawn.BP_Grid` (`self.GridDebugPawn`)))
  (`/Game/Systems/GridSystem/BaseGrid/BFL_GridUtilities.ClearStateFromAllTiles` "NewEnumerator7" (`/Game/Systems/GridSystem/DebugTools/BP_GridDebugPawn.BP_Grid` (`self.GridDebugPawn`)))
  ;;[0 0 0] Gets all of our input tile's valid neighbours from the Grid Pathfinding BP
  (bind _valid_neighbours (`/Game/Systems/GridSystem/Pathfinding/BP_GridPathfinding.Get Valid Tile Neighbours` (`/Game/Systems/GridSystem/BaseGrid/BP_GridManager.Grid_Pathfinding` (`/Game/Systems/GridSystem/DebugTools/BP_GridDebugPawn.BP_Grid` (`self.GridDebugPawn`))) `Tile ID` (`self.Include Diagonals`) (`|MakeArray` "NewEnumerator0" "NewEnumerator11" "NewEnumerator12" "NewEnumerator13" :!type "/Game/Systems/GridSystem/BaseGrid/TileData/EN_TileTerrain Enum")))
  ;;[0 0 0] Adds the IsNeighbour state to all of our target tile's neighbouring tiles
  (for _array_element _valid_neighbours
    (`/Game/Systems/GridSystem/BaseGrid/BFL_GridUtilities.Add State To Tile` (break `/Game/Systems/GridSystem/Pathfinding/ST_PathfindingData` _array_element) "NewEnumerator7" (`/Game/Systems/GridSystem/DebugTools/BP_GridDebugPawn.BP_Grid` (`self.GridDebugPawn`)))))

(fn `UserConstructionScript`
  (`parent.UserConstructionScript`))