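; BP_GridActions is an actor that handles mouse interaction with the tile grid managed by BP_GridManager.
; On BeginPlay it finds the grid manager and enables player input, then checks the tile under the cursor every tick.
; When that tile changes, it moves a hover state from the previous tile to the new one.
; Left click adds a second state to the hovered tile, and right click removes it.
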(event `self.ReceiveBeginPlay`
  (bind _returnvalue (`GameplayStatics.GetActorOfClass` "/Game/Systems/GridSystem/BaseGrid/BP_GridManager.BP_GridManager_C"))
  (set `self.Grid` _returnvalue)
  (`self.EnableInput` (`GameplayStatics.GetPlayerController` 0)))

(event `self.ReceiveTick`
  (params (DeltaSeconds :type "Float (single-precision)"))
  (`self.UpdateTileUnderCursor`))

(event `Key|LeftMouseButton`
  (params (Key :type "Key Structure"))
  (:`Pressed`
    (`/Game/Systems/GridSystem/BaseGrid/BFL_GridUtilities.Add State To Tile` (`self.HoveredTile`) "NewEnumerator2" (`self.Grid`))))

(event `Key|RightMouseButton`
  (params (Key :type "Key Structure"))
  (:`Pressed`
    (`/Game/Systems/GridSystem/BaseGrid/BFL_GridUtilities.Remove State From Tile` (`self.HoveredTile`) "NewEnumerator2" (`self.Grid`))))

(fn `UpdateTileUnderCursor`
  (bind _grid (`self.Grid`))
  (bind _hoveredtile (`self.HoveredTile`))
  (bind _grid_id (`/Game/Systems/GridSystem/BaseGrid/BFL_GridUtilities.Get Tile ID Under Cursor` _grid))
  (if (!= _grid_id _hoveredtile)
    (`/Game/Systems/GridSystem/BaseGrid/BFL_GridUtilities.Remove State From Tile` _hoveredtile "NewEnumerator1" _grid)
    (set `self.HoveredTile` _grid_id)
    (`/Game/Systems/GridSystem/BaseGrid/BFL_GridUtilities.Add State To Tile` (`self.HoveredTile`) "NewEnumerator1" _grid)))

(fn `UserConstructionScript`)