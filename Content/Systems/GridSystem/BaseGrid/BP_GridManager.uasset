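; Grid manager actor that builds a centred, snapped tile grid, storing per-tile data and rendering it through an instanced static mesh.
; Construction script and GenerateGrid clear and rebuild the grid; construction also links a child-actor pathfinding component back to it.
; Tile updates re-add instances, writing priority-ordered state colours into per-instance custom data, and notify listeners.
; Helpers derive walkability from terrain and spawn debug actors for some terrain types.
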(event `GenerateGrid`
  ;[1 1 1] Editor called function that clears the grid and then generates a new grid
  (`self.Clear Grid`)
  (`self.CreateGrid` (`self.K2_GetActorLocation`) (`self.Grid_TileSize`) (`self.Grid_Dimensions`) (make `/Game/Systems/GridSystem/BaseGrid/TileData/ST_TileData` (struct))))

(event `UpdateGrid`)

(fn `Add Tile`
  (params (`Tile Data` :type "/Game/Systems/GridSystem/BaseGrid/TileData/ST_TileData Structure"))
  (`BlueprintMapLibrary.Map_Add` (`self.Tile_Data_Library`) (`.TileID_4_7BEDBA7744FCB1E5F5C164A33CAE4A02` (break `/Game/Systems/GridSystem/BaseGrid/TileData/ST_TileData` `Tile Data`)) `Tile Data`)
  (`self.Update Tile Instance` `Tile Data`))

(fn `CalculateGridCentre&BottomLeft`
  (returns (Centre :type "Vector Structure") (BottomLeft :type "Vector Structure"))
  (locals (C :type "Vector Structure"))
  (bind (_grid_dimensions_x _grid_dimensions_y) (break `IntPoint` (`self.Grid_Dimensions`)))
  (set `local.C` (`/Game/Systems/GridSystem/BaseGrid/BFL_GridUtilities.Snap Vector to Vector` (`self.Grid_Centre_Location`) (`self.Grid_TileSize`)))
  (return (`local.C`) (- (`local.C`) (* (/ (- (`self.Grid_Dimensions`) (`KismetMathLibrary.MakeVector2D` (`KismetMathLibrary.SelectFloat` 0.0 1.0 (`/Game/Systems/GridSystem/BaseGrid/BFL_GridUtilities.Is Int Even?` _grid_dimensions_x)) (`KismetMathLibrary.SelectFloat` 0.0 1.0 (`/Game/Systems/GridSystem/BaseGrid/BFL_GridUtilities.Is Int Even?` _grid_dimensions_y)))) 2.0) (`self.Grid_TileSize`)))))

(fn `Clear Grid`
  ;[1 1 1] Clears all of the mesh instances from the grid and then clears the Tile ID Array
  (`InstancedStaticMeshComponent.ClearInstances` (`self.InstancedGridMesh`))
  (`KismetArrayLibrary.Array_Clear` (`self.InstanceIDs`))
  (`BlueprintMapLibrary.Map_Clear` (`self.Tile_Data_Library`))
  (`self.OnGridDestroyed`))

(fn `CreateGrid`
  (params (Centre_Location :type "Vector Structure") (TileSize :type "Vector Structure") (Dimensions :type "IntPoint Structure") (Tile_Data :type "/Game/Systems/GridSystem/BaseGrid/TileData/ST_TileData Structure"))
  (locals (X :type Integer) (Y :type Integer) (`Current Tile ID` :type "IntPoint Structure"))
  (bind (_grid_dimensions_x _grid_dimensions_y) (break `IntPoint` (`self.Grid_Dimensions`)))
  (bind _grid_dimensions_x_2 (break `IntPoint` (`self.Grid_Dimensions`)))
  ;[1 1 1] Saves variables for later use throughout grid lifespan
  (set `self.Grid_Centre_Location` Centre_Location)
  (set `self.Grid_TileSize` TileSize)
  (set `self.Grid_Dimensions` Dimensions)
  ;[1 1 1] Apply grid offset to stop Z-Fighting
  (`SceneComponent.K2_SetWorldLocation` (`self.InstancedGridMesh`) (`KismetMathLibrary.MakeVector` 0.0 0.0 (`self.Grid_Offset_From_Ground`)) false false)
  ;[1 1 1] Calculates the grid centre offset so the grid is always centred on the gridmanager actor transform
  (bind (_centre _bottomleft) (`self.CalculateGridCentre&BottomLeft`))
  (set `self.Grid_Centre_Location` _centre)
  (set `self.Grid_BottomLeft_Location` _bottomleft)
  ;[1 1 1] Iterates through the X & Y positions of our grid to update each tile's state. Then saves the current tile's X & Y coordinate for storing in the Index
  (for _index (range _grid_dimensions_x_2)
    (set `local.X` _index)
    (for _index_2 (range _grid_dimensions_y)
      (set `local.Y` _index_2)
      ;[1 1 1] Tile ID (This tracks our current progress and selected tile.)
      (bind _output_get (set `local.Current Tile ID` (make `IntPoint` (`local.X`) (`local.Y`))))
      (bind _output_get_2 (set `self.CurrentTileTransform` (`KismetMathLibrary.MakeTransform` (`self.GetTileLocationFromGridIndex` (`local.Current Tile ID`)))))
      (`self.Add Tile` (make `/Game/Systems/GridSystem/BaseGrid/TileData/ST_TileData` _output_get _ _output_get_2)))))

(fn `GetColourFromState`
  (params (States :type "Array of /Game/Systems/GridSystem/BaseGrid/TileData/EN_TileState Enum"))
  (returns (Colour :type "LinearColor Structure") (`IsFilled?` :type "Float (double-precision)"))
  ;[0 0 0] This function is used to set the display colour for each grid square. If you want the function that implements per tile visual changes, that is 'UpdateTileInstance'. If you want grid wide visual changes that is 'InitializeGridMeshVisual'
  ;;[0 0 0] Checks if the current tile has any states assigned to it
  (if (== (`KismetArrayLibrary.Array_Length` States) 0)
    ;;[0 0 0] No, the current tile has no state assigned to it, return without changing
    (return (struct) 0.0)
    (else
      ;;[0 0 0] Cycles through an array of potential states filtered for importance
      (for _array_element (`|MakeArray` "NewEnumerator2" "NewEnumerator1" "NewEnumerator7" "NewEnumerator8" "NewEnumerator9" "NewEnumerator10" :!type "/Game/Systems/GridSystem/BaseGrid/TileData/EN_TileState Enum")
        ;;[0 0 0] We check for the states and return once we hit a state. This is formatted like this so states of higher importance like 'Selected' display instead of 'Hovered. We then Select the corresponding colour for the state
        (if (`KismetArrayLibrary.Array_Contains` States _array_element)
          (return (select `/Game/Systems/GridSystem/BaseGrid/TileData/EN_TileState` _array_element :`NewEnumerator1` (struct :`R` 0.375 :`G` 0.333661 :`B` 0.068359 :`A` 1.0) :`NewEnumerator2` (struct :`R` 1.0 :`G` 0.324505 :`A` 1.0) :`NewEnumerator7` (struct :`R` 0.972319 :`B` 1.0 :`A` 1.0) :`NewEnumerator8` (struct :`R` 0.137853 :`B` 0.375 :`A` 1.0) :`NewEnumerator9` (struct :`R` 0.912414 :`G` 0.169732 :`B` 1.0 :`A` 1.0) :`NewEnumerator10` (struct :`R` 0.248751 :`G` 0.077422 :`B` 0.328125 :`A` 1.0) :!type "LinearColor Structure") 1.0)))
      ;;[0 0 0] None of our specified states have been hit so we return without changes
      (return (struct) 0.0))))

(fn `GetTileLocationFromGridIndex`
  (params (GridIndex :type "IntPoint Structure"))
  (returns (TileLocation :type "Vector Structure"))
  (return (+ (`self.Grid_BottomLeft_Location`) (* (`self.Grid_TileSize`) (`KismetMathLibrary.Conv_IntPointToVector2D` GridIndex)))))

(fn `GetTileRotationFromGridIndex`
  (params (`Grid Index` :type "IntPoint Structure"))
  (returns (`Tile Rotation` :type "Rotator Structure"))
  (return))

(fn `Initialize Grid Mesh Visual`
  (params (Mesh :type "StaticMesh Object Reference") (Material :type "MaterialInterface Object Reference") (Colour :type "LinearColor Structure") (Collision :type "ECollisionEnabled Enum" :default "NoCollision"))
  (`StaticMeshComponent.SetStaticMesh` (`self.InstancedGridMesh`) Mesh)
  (`PrimitiveComponent.SetMaterial` (`self.InstancedGridMesh`) 0 Material)
  (`MeshComponent.SetVectorParameterValueOnMaterials` (`self.InstancedGridMesh`) "Colour" (`KismetMathLibrary.Conv_LinearColorToVector` Colour))
  (`PrimitiveComponent.SetCollisionEnabled` (`self.InstancedGridMesh`) Collision))

(fn `IsTileWalkable`
  (params (`Tile ID` :type "IntPoint Structure"))
  (returns (`IsWalkable?` :type Boolean))
  (bind (_value _returnvalue) (`BlueprintMapLibrary.Map_Find` (`self.Tile_Data_Library`) `Tile ID`))
  (if _returnvalue
    (switch `/Game/Systems/GridSystem/BaseGrid/TileData/EN_TileTerrain` (`.Terrain_24_E629DEFF45AA8E6AB9C870A32B4167DD` (break `/Game/Systems/GridSystem/BaseGrid/TileData/ST_TileData` _value))
      (:`NewEnumerator0`
        _)
      (:`NewEnumerator11`
        _)
      (:`NewEnumerator12`
        _)
      (:`NewEnumerator13`
        _)
      (:`NewEnumerator14`
        (return false))
      (:`NewEnumerator15`
        (return false))
      (:`NewEnumerator16`
        _)
      (:`NewEnumerator17`
        _))
    (return true)
    (else
      (return false))))

(fn `IterateThroughTiles`
  (locals (X :type Integer) (Y :type Integer) (`Current Tile ID` :type "IntPoint Structure"))
  (bind (_grid_dimensions_x _grid_dimensions_y) (break `IntPoint` (`self.Grid_Dimensions`)))
  (bind _grid_dimensions_x_2 (break `IntPoint` (`self.Grid_Dimensions`)))
  (for _index (range _grid_dimensions_x_2)
    (set `local.X` _index)
    (for _index_2 (range _grid_dimensions_y)
      (set `local.Y` _index_2)
      (bind _output_get (set `local.Current Tile ID` (make `IntPoint` (`local.X`) (`local.Y`))))
      (`self.OnTileDataUpdated` _output_get))))

(fn `Remove Tile`
  (params (`ID To Remove` :type "IntPoint Structure (by ref)"))
  (bind _instanceids (`self.InstanceIDs`))
  (if (`KismetArrayLibrary.Array_Contains` _instanceids `ID To Remove`)
    (`InstancedStaticMeshComponent.RemoveInstance` (`self.InstancedGridMesh`) (`KismetArrayLibrary.Array_Find` _instanceids `ID To Remove`))
    (`KismetArrayLibrary.Array_RemoveItem` (`self.InstanceIDs`) `ID To Remove`)
    (`self.OnTileDataUpdated` `ID To Remove`)))

(fn `SpawnMeshAtTileLocation`
  (params (`Tile ID` :type "IntPoint Structure"))
  (bind (_value _returnvalue) (`BlueprintMapLibrary.Map_Find` (`self.Tile_Data_Library`) `Tile ID`))
  (bind (_tileid _tilestates _transform _visited _walkable_ _terrain) (break `/Game/Systems/GridSystem/BaseGrid/TileData/ST_TileData` _value))
  (if _returnvalue
    (switch `/Game/Systems/GridSystem/BaseGrid/TileData/EN_TileTerrain` _terrain
      (:`NewEnumerator11`
        (`|SpawnActorFromClass` "/Game/Systems/GridSystem/DebugTools/VisualAids/BP_DebugRough.BP_DebugRough_C" _transform "AlwaysSpawn" "MultiplyWithRoot" null null))
      (:`NewEnumerator14`
        (`|SpawnActorFromClass` "/Game/Systems/GridSystem/DebugTools/VisualAids/BP_DebugObstacle.BP_DebugObstacle_C" _transform "AlwaysSpawn" "MultiplyWithRoot" null null)))))

(fn `Update Tile Instance`
  (params (`Tile Data` :type "/Game/Systems/GridSystem/BaseGrid/TileData/ST_TileData Structure"))
  (bind _instancedgridmesh (`self.InstancedGridMesh`))
  (`self.Remove Tile` `Tile Data_TileID_4_7BEDBA7744FCB1E5F5C164A33CAE4A02`)
  (`InstancedStaticMeshComponent.AddInstance` (`self.InstancedGridMesh`) `Tile Data_Transform_12_ACB12EFD46E1A6A0191A1C9C09D4F5A4` false)
  (bind _returnvalue (`KismetArrayLibrary.Array_Add` (`self.InstanceIDs`) `Tile Data_TileID_4_7BEDBA7744FCB1E5F5C164A33CAE4A02`))
  (bind (_colour _isfilled_) (`self.GetColourFromState` `Tile Data_TileStates_17_FBA7A2D94507533A1F000EAA1BE3A98A`))
  (`InstancedStaticMeshComponent.SetCustomDataValue` _instancedgridmesh _returnvalue 0 (break `LinearColor` _colour) false)
  (`InstancedStaticMeshComponent.SetCustomDataValue` _instancedgridmesh _returnvalue 1 (`.G` (break `LinearColor` _colour)) false)
  (`InstancedStaticMeshComponent.SetCustomDataValue` _instancedgridmesh _returnvalue 2 (`.B` (break `LinearColor` _colour)) false)
  (`InstancedStaticMeshComponent.SetCustomDataValue` _instancedgridmesh _returnvalue 3 _isfilled_ false)
  (`self.OnTileDataUpdated` `Tile Data_TileID_4_7BEDBA7744FCB1E5F5C164A33CAE4A02`))

(fn `UserConstructionScript`
  ;[0 0 0] We are connecting to the Grid Pathfinding child actor inside the grid. By keeping the Grid Pathfinding to a dedicated child actor, it should help designers with keeping track of different grid components.
  (bind _asbp_grid_pathfinding (cast `/Game/Systems/GridSystem/Pathfinding/BP_GridPathfinding` (`ChildActorComponent.ChildActor` (`self.ChildActor_GridPathfinding`))))
  (bind _output_get (set `self.Grid_Pathfinding` _asbp_grid_pathfinding))
  (set `/Game/Systems/GridSystem/Pathfinding/BP_GridPathfinding.BP_Grid` self _output_get)
  ;[0 0 0] We are clearing our prior grid and creating a new one
  (`self.Clear Grid`)
  (`self.CreateGrid` (`self.K2_GetActorLocation`) (`self.Grid_TileSize`) (`self.Grid_Dimensions`) (make `/Game/Systems/GridSystem/BaseGrid/TileData/ST_TileData` (struct))))