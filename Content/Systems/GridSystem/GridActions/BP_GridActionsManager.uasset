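; BP_GridActionsManager tracks the grid tile under the cursor and manages the actions selected for left and right click.
; Every tick it asks BP_GridManager for the cursor's tile and moves a tile state from the old tile to the new one on change.
; SetSelectedActions replaces each click's action by destroying the old actor and spawning one from the given class with a back-reference.
; Both clicks start as BP_Action_SelectTile.
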(event `self.ReceiveBeginPlay`
  (bind _returnvalue (`GameplayStatics.GetActorOfClass` "/Game/Systems/GridSystem/BaseGrid/BP_GridManager.BP_GridManager_C"))
  (set `self.Grid` _returnvalue)
  (`self.EnableInput` (`GameplayStatics.GetPlayerController` 0))
  (`self.SetSelectedActions` "/Game/Systems/GridSystem/GridActions/BP_Action_SelectTile.BP_Action_SelectTile_C" "/Game/Systems/GridSystem/GridActions/BP_Action_SelectTile.BP_Action_SelectTile_C"))

(event `self.ReceiveTick`
  (params (DeltaSeconds :type "Float (single-precision)"))
  (`self.UpdateTileUnderCursor`))

(event `Key|LeftMouseButton`
  (params (Key :type "Key Structure")))

(event `Key|RightMouseButton`
  (params (Key :type "Key Structure")))

(fn `SetSelectedActions`
  (params (`Left Action` :type "/Game/Systems/GridSystem/GridActions/BP_Action Class Reference") (`Right Action` :type "/Game/Systems/GridSystem/GridActions/BP_Action Class Reference"))
  (bind _selectedaction_rightclick (`self.SelectedAction_RightClick`))
  (bind _selectedaction_leftclick (`self.SelectedAction_LeftClick`))
  (`|ExecutionSequence`
    (:`then_0`
      ;[1 1 1] Checks and deletes prior selected action so we are ready for our new action
      (`/Engine/EditorBlueprintResources/StandardMacros.IsValid` _selectedaction_leftclick
        (:`Is Valid`
          (`self.K2_DestroyActor` _selectedaction_leftclick)
          (set `self.SelectedAction_LeftClick` null))
        (:`Is Not Valid`
          _))
      ;[1 1 1] Checks if our left action class is valid and then spawns in an action actor to assign as Selected Action Left Click
      (if (`KismetSystemLibrary.IsValidClass` (`local.Left Action`))
        (bind _returnvalue (`|SpawnActorFromClass` (`local.Left Action`) (`KismetMathLibrary.MakeTransform` (0.0 0.0 0.0)) "AlwaysSpawn" "MultiplyWithRoot" null self null))
        (set `self.SelectedAction_LeftClick` _returnvalue)))
    (:`then_1`
      ;[1 1 1] Checks and deletes prior selected action so we are ready for our new action
      (`/Engine/EditorBlueprintResources/StandardMacros.IsValid` _selectedaction_rightclick
        (:`Is Valid`
          (`self.K2_DestroyActor` _selectedaction_rightclick)
          (set `self.SelectedAction_RightClick` null))
        (:`Is Not Valid`
          _))
      ;[1 1 1] Checks if our right action class is valid and then spawns in an action actor to assign as Selected Action right Click
      (if (`KismetSystemLibrary.IsValidClass` (`local.Right Action`))
        (bind _returnvalue_2 (`|SpawnActorFromClass` (`local.Right Action`) (`KismetMathLibrary.MakeTransform` (0.0 0.0 0.0)) "AlwaysSpawn" "MultiplyWithRoot" null self null))
        (set `self.SelectedAction_RightClick` _returnvalue_2)))))

(fn `UpdateTileUnderCursor`
  (bind _grid (`self.Grid`))
  (bind _hoveredtile (`self.HoveredTile`))
  (bind _grid_id (`/Game/Systems/GridSystem/BaseGrid/BFL_GridUtilities.Get Tile ID Under Cursor` _grid))
  (if (!= _grid_id _hoveredtile)
    (`/Game/Systems/GridSystem/BaseGrid/BFL_GridUtilities.Remove State From Tile` _hoveredtile "NewEnumerator1" _grid)
    (set `self.HoveredTile` _grid_id)
    (`/Game/Systems/GridSystem/BaseGrid/BFL_GridUtilities.Add State To Tile` (`self.HoveredTile`) "NewEnumerator1" _grid)))

(fn `UserConstructionScript`)