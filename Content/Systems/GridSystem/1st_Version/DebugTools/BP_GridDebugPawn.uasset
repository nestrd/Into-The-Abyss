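; Debug pawn for the grid system, providing a controllable camera and mouse-driven tools for selecting tiles, showing neighbours, finding paths and editing terrain.
; Zoom, movement and rotation inputs set desired values that Tick interpolates toward, while also updating the hovered tile.
; Tool keys respawn left and right action actors through SetSelectedActions.
; Clicks execute the matching action on the hovered tile, so each tool's logic lives in its own actor.
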(event `self.ReceiveBeginPlay`
  (bind _returnvalue (`GameplayStatics.GetActorOfClass` "/Game/Systems/GridSystem/1st_Version/BaseGrid/BP_GridManager.BP_GridManager_C"))
  (set `self.BP_Grid` _returnvalue)
  (set `self.Location_Desired` (`self.K2_GetActorLocation`))
  (set `self.Zoom_Desired` (`SpringArmComponent.TargetArmLength` (`self.CameraSpring`)))
  (set `self.Rotation_Desired` (`self.K2_GetActorRotation`))
  (bind _returnvalue_2 (`GameplayStatics.GetActorOfClass` "/Game/Systems/GridSystem/1st_Version/DebugTools/VisualAids/BP_DebugTextAndColoursOnTiles.BP_DebugTextAndColoursOnTiles_C"))
  (set `self.DebugTextOnTiles` _returnvalue_2)
  (`self.SetSelectedActions` "/Game/Systems/GridSystem/GridActions/BP_Action_SelectTile.BP_Action_SelectTile_C" "/Game/Systems/GridSystem/GridActions/BP_Action_SelectTile.BP_Action_SelectTile_C"))

(event `EnhancedInput|/Game/Systems/GridSystem/1st_Version/DebugTools/DebugInputs/InputActions/GIA_Tool1`
  (params (ActionValue :type Boolean) (ElapsedSeconds :type "Float (double-precision)") (TriggeredSeconds :type "Float (double-precision)") (InputAction :type "InputAction Object Reference" :default "/Game/Systems/GridSystem/1st_Version/DebugTools/DebugInputs/InputActions/GIA_Tool1.GIA_Tool1"))
  (:`Started`
    (`self.SetSelectedActions` "/Game/Systems/GridSystem/GridActions/BP_Action_SelectTile.BP_Action_SelectTile_C" "/Game/Systems/GridSystem/GridActions/BP_Action_SelectTile.BP_Action_SelectTile_C")))

(event `EnhancedInput|/Game/Systems/GridSystem/1st_Version/DebugTools/DebugInputs/InputActions/GIA_Zoom`
  (params (ActionValue :type "Float (double-precision)") (ElapsedSeconds :type "Float (double-precision)") (TriggeredSeconds :type "Float (double-precision)") (InputAction :type "InputAction Object Reference" :default "/Game/Systems/GridSystem/1st_Version/DebugTools/DebugInputs/InputActions/GIA_Zoom.GIA_Zoom"))
  ;[1 1 1] Zoom logic
  (:`Triggered`
    (set `self.Zoom_Desired` (`KismetMathLibrary.FClamp` (+ (* ActionValue (`self.Zoom_Speed`)) (`self.Zoom_Desired`)) (`self.Zoom_Min`) (`self.Zoom_Max`)))))

(event `EnhancedInput|/Game/Systems/GridSystem/1st_Version/DebugTools/DebugInputs/InputActions/GIA_Tool2`
  (params (ActionValue :type Boolean) (ElapsedSeconds :type "Float (double-precision)") (TriggeredSeconds :type "Float (double-precision)") (InputAction :type "InputAction Object Reference" :default "/Game/Systems/GridSystem/1st_Version/DebugTools/DebugInputs/InputActions/GIA_Tool2.GIA_Tool2"))
  (:`Started`
    (`self.SetSelectedActions` "/Game/Systems/GridSystem/Pathfinding/BP_Action_ShowTileNeighbours.BP_Action_ShowTileNeighbours_C" "/Game/Systems/GridSystem/Pathfinding/BP_Action_ShowTileNeighbours.BP_Action_ShowTileNeighbours_C")))

(event `EnhancedInput|/Game/Systems/GridSystem/1st_Version/DebugTools/DebugInputs/InputActions/GIA_Forwards`
  (params (ActionValue :type "Float (double-precision)") (ElapsedSeconds :type "Float (double-precision)") (TriggeredSeconds :type "Float (double-precision)") (InputAction :type "InputAction Object Reference" :default "/Game/Systems/GridSystem/1st_Version/DebugTools/DebugInputs/InputActions/GIA_Forwards.GIA_Forwards"))
  ;[1 1 1] Movement Logic
  (:`Triggered`
    (set `self.Location_Desired` (+ (* (* ActionValue (`self.Location_Speed`)) (`self.GetActorForwardVector`)) (`self.Location_Desired`)))))

(event `EnhancedInput|/Game/Systems/GridSystem/1st_Version/DebugTools/DebugInputs/InputActions/GIA_Tool3`
  (params (ActionValue :type Boolean) (ElapsedSeconds :type "Float (double-precision)") (TriggeredSeconds :type "Float (double-precision)") (InputAction :type "InputAction Object Reference" :default "/Game/Systems/GridSystem/1st_Version/DebugTools/DebugInputs/InputActions/GIA_Tool3.GIA_Tool3"))
  (:`Started`
    (`self.SetSelectedActions` "/Game/Systems/GridSystem/Pathfinding/BP_Action_FindPathToTarget.BP_Action_FindPathToTarget_C" "/Game/Systems/GridSystem/Pathfinding/BP_Action_FindPathToTarget.BP_Action_FindPathToTarget_C")))

(event `EnhancedInput|/Game/Systems/GridSystem/1st_Version/DebugTools/DebugInputs/InputActions/GIA_Sideways`
  (params (ActionValue :type "Float (double-precision)") (ElapsedSeconds :type "Float (double-precision)") (TriggeredSeconds :type "Float (double-precision)") (InputAction :type "InputAction Object Reference" :default "/Game/Systems/GridSystem/1st_Version/DebugTools/DebugInputs/InputActions/GIA_Sideways.GIA_Sideways"))
  ;[1 1 1] Movement Logic
  (:`Triggered`
    (set `self.Location_Desired` (+ (* (* ActionValue (`self.Location_Speed`)) (`self.GetActorRightVector`)) (`self.Location_Desired`)))))

(event `EnhancedInput|/Game/Systems/GridSystem/1st_Version/DebugTools/DebugInputs/InputActions/GIA_Tool4`
  (params (ActionValue :type Boolean) (ElapsedSeconds :type "Float (double-precision)") (TriggeredSeconds :type "Float (double-precision)") (InputAction :type "InputAction Object Reference" :default "/Game/Systems/GridSystem/1st_Version/DebugTools/DebugInputs/InputActions/GIA_Tool4.GIA_Tool4"))
  (:`Started`
    (`self.SetSelectedActions` "/Game/Systems/GridSystem/GridActions/BP_Action_SetNormalTerrain.BP_Action_SetNormalTerrain_C" "/Game/Systems/GridSystem/GridActions/BP_Action_SetNormalTerrain.BP_Action_SetNormalTerrain_C")))

(event `EnhancedInput|/Game/Systems/GridSystem/1st_Version/DebugTools/DebugInputs/InputActions/GIA_RotateRight`
  (params (ActionValue :type Boolean) (ElapsedSeconds :type "Float (double-precision)") (TriggeredSeconds :type "Float (double-precision)") (InputAction :type "InputAction Object Reference" :default "/Game/Systems/GridSystem/1st_Version/DebugTools/DebugInputs/InputActions/GIA_RotateRight.GIA_RotateRight"))
  ;[1 1 1] Rotate Camera
  (:`Started`
    (set `self.Rotation_Desired` (`KismetMathLibrary.ComposeRotators` (`self.Rotation_Desired`) (`KismetMathLibrary.MakeRotator` 0.0 0.0 (- 0.0 (`self.Rotation_Speed`)))))))

(event `EnhancedInput|/Game/Systems/GridSystem/1st_Version/DebugTools/DebugInputs/InputActions/GIA_Tool5`
  (params (ActionValue :type Boolean) (ElapsedSeconds :type "Float (double-precision)") (TriggeredSeconds :type "Float (double-precision)") (InputAction :type "InputAction Object Reference" :default "/Game/Systems/GridSystem/1st_Version/DebugTools/DebugInputs/InputActions/GIA_Tool5.GIA_Tool5"))
  (:`Started`
    (`self.SetSelectedActions` "/Game/Systems/GridSystem/GridActions/BP_Action_SetRoughTerrain.BP_Action_SetRoughTerrain_C" "/Game/Systems/GridSystem/GridActions/BP_Action_SetNormalTerrain.BP_Action_SetNormalTerrain_C")))

(event `EnhancedInput|/Game/Systems/GridSystem/1st_Version/DebugTools/DebugInputs/InputActions/GIA_Tool6`
  (params (ActionValue :type Boolean) (ElapsedSeconds :type "Float (double-precision)") (TriggeredSeconds :type "Float (double-precision)") (InputAction :type "InputAction Object Reference" :default "/Game/Systems/GridSystem/1st_Version/DebugTools/DebugInputs/InputActions/GIA_Tool6.GIA_Tool6"))
  (:`Started`
    (`self.SetSelectedActions` "/Game/Systems/GridSystem/GridActions/BP_Action_SetObstacle.BP_Action_SetObstacle_C" "/Game/Systems/GridSystem/GridActions/BP_Action_SetNormalTerrain.BP_Action_SetNormalTerrain_C")))

(event `EnhancedInput|/Game/Systems/GridSystem/1st_Version/DebugTools/DebugInputs/InputActions/GIA_RotateLeft`
  (params (ActionValue :type Boolean) (ElapsedSeconds :type "Float (double-precision)") (TriggeredSeconds :type "Float (double-precision)") (InputAction :type "InputAction Object Reference" :default "/Game/Systems/GridSystem/1st_Version/DebugTools/DebugInputs/InputActions/GIA_RotateLeft.GIA_RotateLeft"))
  ;[1 1 1] Rotate Camera
  (:`Started`
    (set `self.Rotation_Desired` (`KismetMathLibrary.ComposeRotators` (`self.Rotation_Desired`) (`KismetMathLibrary.MakeRotator` 0.0 0.0 (`self.Rotation_Speed`))))))

(event `self.ReceiveTick`
  (params (DeltaSeconds :type "Float (single-precision)"))
  (bind _cameraspring (`self.CameraSpring`))
  (set `SpringArmComponent.TargetArmLength` (`KismetMathLibrary.FInterpTo` (`SpringArmComponent.TargetArmLength` _cameraspring) (`self.Zoom_Desired`) DeltaSeconds (`self.Zoom_Interp`)) _cameraspring)
  (`self.K2_SetActorLocation` (`KismetMathLibrary.VInterpTo` (`self.K2_GetActorLocation`) (`self.Location_Desired`) DeltaSeconds (`self.Location_Interp`)))
  (`self.K2_SetActorRotation` (`KismetMathLibrary.RInterpTo` (`self.K2_GetActorRotation`) (`self.Rotation_Desired`) DeltaSeconds (`self.Rotation_Interp`)))
  (bind _uptodate_hovered_tile (`/Game/Systems/GridSystem/1st_Version/BaseGrid/BFL_GridUtilities.UpdateTileUnderCursor` (`self.BP_Grid`) "NewEnumerator1" (`self.HoveredTile`)))
  (set `self.HoveredTile` _uptodate_hovered_tile))

(event `EnhancedInput|/Game/Systems/GridSystem/1st_Version/DebugTools/DebugInputs/InputActions/GIA_LeftClick`
  (params (ActionValue :type Boolean) (ElapsedSeconds :type "Float (double-precision)") (TriggeredSeconds :type "Float (double-precision)") (InputAction :type "InputAction Object Reference" :default "/Game/Systems/GridSystem/1st_Version/DebugTools/DebugInputs/InputActions/GIA_LeftClick.GIA_LeftClick"))
  (:`Started`
    (`/Engine/EditorBlueprintResources/StandardMacros.IsValid` (`self.SelectedAction_LeftClick`)
      (:`Is Valid`
        (`/Game/Systems/GridSystem/GridActions/BP_Action.Execute Action` (`self.SelectedAction_LeftClick`) (`self.HoveredTile`))))))

(event `EnhancedInput|/Game/Systems/GridSystem/1st_Version/DebugTools/DebugInputs/InputActions/GIA_RightClick`
  (params (ActionValue :type Boolean) (ElapsedSeconds :type "Float (double-precision)") (TriggeredSeconds :type "Float (double-precision)") (InputAction :type "InputAction Object Reference" :default "/Game/Systems/GridSystem/1st_Version/DebugTools/DebugInputs/InputActions/GIA_RightClick.GIA_RightClick"))
  (:`Started`
    (`/Engine/EditorBlueprintResources/StandardMacros.IsValid` (`self.SelectedAction_RightClick`)
      (:`Is Valid`
        (`/Game/Systems/GridSystem/GridActions/BP_Action.Execute Action` (`self.SelectedAction_RightClick`) (`self.HoveredTile`))))))

(fn `SetSelectedActions`
  (params (`Left Action` :type "/Game/Systems/GridSystem/GridActions/BP_Action Class Reference") (`Right Action` :type "/Game/Systems/GridSystem/GridActions/BP_Action Class Reference"))
  (bind _selectedaction_rightclick (`self.SelectedAction_RightClick`))
  (bind _selectedaction_leftclick (`self.SelectedAction_LeftClick`))
  (`|ExecutionSequence`
    (:`then_0`
      ;[1 1 1] Checks and deletes prior selected action so we are ready for our new action
      (`/Engine/EditorBlueprintResources/StandardMacros.IsValid` _selectedaction_leftclick
        (:`Is Valid`
          (`self.K2_DestroyActor` _selectedaction_leftclick)
          (set `self.SelectedAction_LeftClick` null))
        (:`Is Not Valid`
          _))
      ;[1 1 1] Checks if our left action class is valid and then spawns in an action actor to assign as Selected Action Left Click
      (if (`KismetSystemLibrary.IsValidClass` (`local.Left Action`))
        (bind _returnvalue (`|SpawnActorFromClass` (`local.Left Action`) (`KismetMathLibrary.MakeTransform` (0.0 0.0 0.0)) "AlwaysSpawn" "MultiplyWithRoot" null self null))
        (set `self.SelectedAction_LeftClick` _returnvalue)))
    (:`then_1`
      ;[1 1 1] Checks and deletes prior selected action so we are ready for our new action
      (`/Engine/EditorBlueprintResources/StandardMacros.IsValid` _selectedaction_rightclick
        (:`Is Valid`
          (`self.K2_DestroyActor` _selectedaction_rightclick)
          (set `self.SelectedAction_RightClick` null))
        (:`Is Not Valid`
          _))
      ;[1 1 1] Checks if our right action class is valid and then spawns in an action actor to assign as Selected Action right Click
      (if (`KismetSystemLibrary.IsValidClass` (`local.Right Action`))
        (bind _returnvalue_2 (`|SpawnActorFromClass` (`local.Right Action`) (`KismetMathLibrary.MakeTransform` (0.0 0.0 0.0)) "AlwaysSpawn" "MultiplyWithRoot" null self null))
        (set `self.SelectedAction_RightClick` _returnvalue_2)))))

(fn `UserConstructionScript`)