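; BP_Action_SelectTile is a grid action that toggles which tile is selected on the grid debug pawn.
; Execute Action first clears two other tile states across the whole grid.
; A new tile ID moves the selected state from the previous tile to that tile and stores it in the pawn's SelectedTile.
; Picking the same tile again removes the state and resets SelectedTile to an invalid sentinel ID.
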(fn `Execute Action`
  (params (`Tile ID` :type "IntPoint Structure"))
  (bind _griddebugpawn (`self.GridDebugPawn`))
  (bind _griddebugpawn_2 (`self.GridDebugPawn`))
  (bind _griddebugpawn_3 (`self.GridDebugPawn`))
  ;[1 1 1] Checks that we are selecting a new tile
  (`/Game/Systems/GridSystem/1st_Version/BaseGrid/BFL_GridUtilities.ClearStateFromAllTiles` "NewEnumerator7" (`/Game/Systems/GridSystem/1st_Version/DebugTools/BP_GridDebugPawn.BP_Grid` _griddebugpawn_2))
  (`/Game/Systems/GridSystem/1st_Version/BaseGrid/BFL_GridUtilities.ClearStateFromAllTiles` "NewEnumerator8" (`/Game/Systems/GridSystem/1st_Version/DebugTools/BP_GridDebugPawn.BP_Grid` _griddebugpawn_2))
  (if (!= (`/Game/Systems/GridSystem/1st_Version/DebugTools/BP_GridDebugPawn.SelectedTile` _griddebugpawn_2) `Tile ID`)
    ;[1 1 1] Removes Selected state from previously selected tile
    (`/Game/Systems/GridSystem/1st_Version/BaseGrid/BFL_GridUtilities.Remove State From Tile` (`/Game/Systems/GridSystem/1st_Version/DebugTools/BP_GridDebugPawn.SelectedTile` _griddebugpawn) "NewEnumerator2" (`/Game/Systems/GridSystem/1st_Version/DebugTools/BP_GridDebugPawn.BP_Grid` _griddebugpawn))
    ;[1 1 1] Updates the Selected Tile variable to be our input Tile ID
    (bind _output_get (set `/Game/Systems/GridSystem/1st_Version/DebugTools/BP_GridDebugPawn.SelectedTile` (`local.Tile ID`) (`self.GridDebugPawn`)))
    ;[1 1 1] Adds the selected state to the current selected tile variable
    (`/Game/Systems/GridSystem/1st_Version/BaseGrid/BFL_GridUtilities.Add State To Tile` _output_get "NewEnumerator2" (`/Game/Systems/GridSystem/1st_Version/DebugTools/BP_GridDebugPawn.BP_Grid` (`self.GridDebugPawn`)))
    (else
      ;[1 1 1] Removes the Selected state from the previously selected tile because the player has selected it again
      (`/Game/Systems/GridSystem/1st_Version/BaseGrid/BFL_GridUtilities.Remove State From Tile` (`/Game/Systems/GridSystem/1st_Version/DebugTools/BP_GridDebugPawn.SelectedTile` _griddebugpawn_3) "NewEnumerator2" (`/Game/Systems/GridSystem/1st_Version/DebugTools/BP_GridDebugPawn.BP_Grid` _griddebugpawn_3))
      ;[1 1 1] Sets the Selected tile variable to an invalid ID
      (set `/Game/Systems/GridSystem/1st_Version/DebugTools/BP_GridDebugPawn.SelectedTile` (make `IntPoint` -999 -999) (`self.GridDebugPawn`)))))

(fn `UserConstructionScript`
  (`parent.UserConstructionScript`))