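; Game mode for real-time gameplay that sets up display, input and the starting character when play begins.
; BeginPlay enables VSync, lowers screen percentage and upscale quality through console commands, and shows the cursor in Game and UI input mode.
; It then calls StartTurn on the first Character_Base tagged PlayerCharacter.
; The GI_PersistentData game instance is cast but not otherwise used.
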(event `self.ReceiveBeginPlay`
  (bind _returnvalue (`GameplayStatics.GetPlayerController` 0))
  (bind _returnvalue_2 (`GameUserSettings.GetGameUserSettings`))
  (`GameUserSettings.SetVSyncEnabled` _returnvalue_2 true)
  (set `self.As GI Persistent Data` (cast `/Game/Systems/GameData/GI_PersistentData` (`GameplayStatics.GetGameInstance`) :!pure true))
  (`KismetSystemLibrary.ExecuteConsoleCommand` "r.ScreenPercentage 75" null)
  (`KismetSystemLibrary.ExecuteConsoleCommand` "r.Upscale.Quality 0" null)
  (`WidgetBlueprintLibrary.SetInputMode_GameAndUIEx` _returnvalue null "DoNotLock" false)
  (set `PlayerController.bShowMouseCursor` true _returnvalue)
  (bind _outactors (`GameplayStatics.GetAllActorsOfClassWithTag` "/Game/Characters/Character_Base.Character_Base_C" "PlayerCharacter"))
  (`/Game/Characters/Character_Base.StartTurn` (`|GetArrayItem` _outactors)))

(fn `UserConstructionScript`)