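; Game mode for turn-based gameplay that gathers all characters and cycles turns between them.
; On begin play it caches the persistent data game instance, lowers render resolution via console commands and shows the mouse cursor.
; It builds the turn order from tagged Character_Base actors, players before NPCs, then starts the first turn and loads every character's deck.
; NextTurn advances the index, wrapping to the first character.
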(event `self.ReceiveBeginPlay`
  (set `self.persistentData` (cast `/Game/Systems/GI_PersistentData` (`GameplayStatics.GetGameInstance`) :!pure true))
  (`KismetSystemLibrary.ExecuteConsoleCommand` "r.ScreenPercentage 75" null)
  (`KismetSystemLibrary.ExecuteConsoleCommand` "r.Upscale.Quality 0" null)
  (set `PlayerController.bShowMouseCursor` true (`GameplayStatics.GetPlayerController` 0))
  (`self.GetAllCharacters`))

(event `GetAllCharacters`
  (bind _outactors (`GameplayStatics.GetAllActorsOfClassWithTag` "/Game/Characters/Character_Base.Character_Base_C" "PlayerCharacter"))
  (for _array_element _outactors
    (`KismetArrayLibrary.Array_Add` (`self.currentCharacters`) _array_element))
  (bind _outactors_2 (`GameplayStatics.GetAllActorsOfClassWithTag` "/Game/Characters/Character_Base.Character_Base_C" "NPCharacter"))
  (for _array_element_2 _outactors_2
    (`KismetArrayLibrary.Array_Add` (`self.currentCharacters`) _array_element_2))
  (`self.StartGame`))

(event `StartGame`
  (bind _currentcharacters (`self.currentCharacters`))
  (`/Game/Characters/Character_Base.StartTurn` (`|GetArrayItem` _currentcharacters))
  (for _array_element _currentcharacters
    (`/Game/Characters/Character_Base.LoadDeck` _array_element)))

(event `NextTurn`
  (bind _result (`/Engine/EditorBlueprintResources/StandardMacros.IncrementInt` (`self.currentTurn`))
    (:`  `
      (bind _output_get (set `self.currentTurn` (select `bool` (>= _result (`KismetArrayLibrary.Array_Length` (`self.currentCharacters`))) :`false` _result)))
      (`/Game/Characters/Character_Base.StartTurn` (`|GetArrayItem` (`self.currentCharacters`) _output_get)))))

(fn `UserConstructionScript`)