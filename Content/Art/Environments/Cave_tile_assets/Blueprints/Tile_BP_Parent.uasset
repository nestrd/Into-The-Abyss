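; Parent Blueprint for cave environment tiles that sets its Cube mesh from TileValue and TileTheme.
; For Default Caves, the construction script maps TileValue to a tile mesh using keys matching a 47-piece, 8-neighbour bitmask autotile set, while Not Default Caves only prints a warning.
; BeginPlay randomizes TileTheme without updating the mesh.
; TileValue is not computed here.
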(event `self.ReceiveBeginPlay`
  ;[1 1 1] Replace BeginPlay with custom event when level opens.
  (set `self.TileTheme` (cast `/Game/Art/Environments/Cave_tile_assets/E_TileTheme` (`KismetMathLibrary.Conv_IntToByte` (`KismetMathLibrary.RandomIntegerInRange` 0 1)))))

(fn `UserConstructionScript`
  (switch `/Game/Art/Environments/Cave_tile_assets/E_TileTheme` (`self.TileTheme`)
    (:`NewEnumerator0`
      (`StaticMeshComponent.SetStaticMesh` (`self.Cube`) (select `/Game/Art/Environments/Cave_tile_assets/E_TileValue` (`self.TileValue`) :`NewEnumerator0` "/Game/Art/Environments/Tile_Sets/Caves_Default/Tile_set_Tile_0.Tile_set_Tile_0" :`NewEnumerator1` "/Game/Art/Environments/Tile_Sets/Caves_Default/Tile_set_Tile_1.Tile_set_Tile_1" :`NewEnumerator2` "/Game/Art/Environments/Tile_Sets/Caves_Default/Tile_set_Tile_4.Tile_set_Tile_4" :`NewEnumerator3` "/Game/Art/Environments/Tile_Sets/Caves_Default/Tile_set_Tile_16.Tile_set_Tile_16" :`NewEnumerator4` "/Game/Art/Environments/Tile_Sets/Caves_Default/Tile_set_Tile_64.Tile_set_Tile_64" :`NewEnumerator5` "/Game/Art/Environments/Tile_Sets/Caves_Default/Tile_set_Tile_5.Tile_set_Tile_5" :`NewEnumerator6` "/Game/Art/Environments/Tile_Sets/Caves_Default/Tile_set_Tile_20.Tile_set_Tile_20" :`NewEnumerator7` "/Game/Art/Environments/Tile_Sets/Caves_Default/Tile_set_Tile_80.Tile_set_Tile_80" :`NewEnumerator8` "/Game/Art/Environments/Tile_Sets/Caves_Default/Tile_set_Tile_65.Tile_set_Tile_65" :`NewEnumerator9` "/Game/Art/Environments/Tile_Sets/Caves_Default/Tile_set_Tile_7.Tile_set_Tile_7" :`NewEnumerator10` "/Game/Art/Environments/Tile_Sets/Caves_Default/Tile_set_Tile_28.Tile_set_Tile_28" :`NewEnumerator11` "/Game/Art/Environments/Tile_Sets/Caves_Default/Tile_set_Tile_112.Tile_set_Tile_112" :`NewEnumerator12` "/Game/Art/Environments/Tile_Sets/Caves_Default/Tile_set_Tile_193.Tile_set_Tile_193" :`NewEnumerator13` "/Game/Art/Environments/Tile_Sets/Caves_Default/Tile_set_Tile_17.Tile_set_Tile_17" :`NewEnumerator14` "/Game/Art/Environments/Tile_Sets/Caves_Default/Tile_set_Tile_68.Tile_set_Tile_68" :`NewEnumerator15` "/Game/Art/Environments/Tile_Sets/Caves_Default/Tile_set_Tile_21.Tile_set_Tile_21" :`NewEnumerator16` "/Game/Art/Environments/Tile_Sets/Caves_Default/Tile_set_Tile_84.Tile_set_Tile_84" :`NewEnumerator17` "/Game/Art/Environments/Tile_Sets/Caves_Default/Tile_set_Tile_81.Tile_set_Tile_81" :`NewEnumerator18` "/Game/Art/Environments/Tile_Sets/Caves_Default/Tile_set_Tile_69.Tile_set_Tile_69" :`NewEnumerator19` "/Game/Art/Environments/Tile_Sets/Caves_Default/Tile_set_Tile_23.Tile_set_Tile_23" :`NewEnumerator20` "/Game/Art/Environments/Tile_Sets/Caves_Default/Tile_set_Tile_92.Tile_set_Tile_92" :`NewEnumerator21` "/Game/Art/Environments/Tile_Sets/Caves_Default/Tile_set_Tile_113.Tile_set_Tile_113" :`NewEnumerator22` "/Game/Art/Environments/Tile_Sets/Caves_Default/Tile_set_Tile_197.Tile_set_Tile_197" :`NewEnumerator23` "/Game/Art/Environments/Tile_Sets/Caves_Default/Tile_set_Tile_29.Tile_set_Tile_29" :`NewEnumerator24` "/Game/Art/Environments/Tile_Sets/Caves_Default/Tile_set_Tile_116.Tile_set_Tile_116" :`NewEnumerator25` "/Game/Art/Environments/Tile_Sets/Caves_Default/Tile_set_Tile_209.Tile_set_Tile_209" :`NewEnumerator26` "/Game/Art/Environments/Tile_Sets/Caves_Default/Tile_set_Tile_71.Tile_set_Tile_71" :`NewEnumerator27` "/Game/Art/Environments/Tile_Sets/Caves_Default/Tile_set_Tile_31.Tile_set_Tile_31" :`NewEnumerator28` "/Game/Art/Environments/Tile_Sets/Caves_Default/Tile_set_Tile_124.Tile_set_Tile_124" :`NewEnumerator29` "/Game/Art/Environments/Tile_Sets/Caves_Default/Tile_set_Tile_241.Tile_set_Tile_241" :`NewEnumerator30` "/Game/Art/Environments/Tile_Sets/Caves_Default/Tile_set_Tile_199.Tile_set_Tile_199" :`NewEnumerator31` "/Game/Art/Environments/Tile_Sets/Caves_Default/Tile_set_Tile_85.Tile_set_Tile_85" :`NewEnumerator32` "/Game/Art/Environments/Tile_Sets/Caves_Default/Tile_set_Tile_87.Tile_set_Tile_87" :`NewEnumerator33` "/Game/Art/Environments/Tile_Sets/Caves_Default/Tile_set_Tile_93.Tile_set_Tile_93" :`NewEnumerator34` "/Game/Art/Environments/Tile_Sets/Caves_Default/Tile_set_Tile_117.Tile_set_Tile_117" :`NewEnumerator35` "/Game/Art/Environments/Tile_Sets/Caves_Default/Tile_set_Tile_213.Tile_set_Tile_213" :`NewEnumerator36` "/Game/Art/Environments/Tile_Sets/Caves_Default/Tile_set_Tile_95.Tile_set_Tile_95" :`NewEnumerator37` "/Game/Art/Environments/Tile_Sets/Caves_Default/Tile_set_Tile_125.Tile_set_Tile_125" :`NewEnumerator38` "/Game/Art/Environments/Tile_Sets/Caves_Default/Tile_set_Tile_245.Tile_set_Tile_245" :`NewEnumerator39` "/Game/Art/Environments/Tile_Sets/Caves_Default/Tile_set_Tile_215.Tile_set_Tile_215" :`NewEnumerator40` "/Game/Art/Environments/Tile_Sets/Caves_Default/Tile_set_Tile_119.Tile_set_Tile_119" :`NewEnumerator41` "/Game/Art/Environments/Tile_Sets/Caves_Default/Tile_set_Tile_221.Tile_set_Tile_221" :`NewEnumerator42` "/Game/Art/Environments/Tile_Sets/Caves_Default/Tile_set_Tile_127.Tile_set_Tile_127" :`NewEnumerator43` "/Game/Art/Environments/Tile_Sets/Caves_Default/Tile_set_Tile_253.Tile_set_Tile_253" :`NewEnumerator44` "/Game/Art/Environments/Tile_Sets/Caves_Default/Tile_set_Tile_247.Tile_set_Tile_247" :`NewEnumerator45` "/Game/Art/Environments/Tile_Sets/Caves_Default/Tile_set_Tile_223.Tile_set_Tile_223" :`NewEnumerator46` "/Game/Art/Environments/Tile_Sets/Caves_Default/Tile_set_Tile_255.Tile_set_Tile_255" :!type "StaticMesh Object Reference")))
    (:`NewEnumerator1`
      (`KismetSystemLibrary.PrintString` "No Tiles Selected" true true (struct :`G` 0.66 :`B` 1.0 :`A` 1.0) 10.0))))